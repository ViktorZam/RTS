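; RTS HUD that handles drag-box unit selection with the mouse.
; Tap, hold and release events clear the previous selection, track the box corners, then pass the selected actors to RTSPlayerController.
; While dragging, DrawHUD draws the box and accumulates Characters inside it that implement SelectionInterface, notifying them and marking them with debug points.
; Leftover debug nodes sit unconnected in the event graph.
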(event Custom|DrawMouseSelection
  (bind _ontapmouseposition__ (Variables|Default|GetOnTapMousePosition%20	))
  (bind _holdingmouseposition (Variables|Default|GetHoldingMousePosition))
  (bind _ontapmouseposition___2 (Variables|Default|GetOnTapMousePosition%20	))
  (bind _ontapmouseposition___3 (Variables|Default|GetOnTapMousePosition%20	))
  (bind _holdingmouseposition_2 (Variables|Default|GetHoldingMousePosition))
  (bind (_x _y) (Math|Vector2D|BreakVector2D _ontapmouseposition___3))
  (bind (_x_2 _y_2) (Math|Vector2D|BreakVector2D _ontapmouseposition__))
  (bind (_x_3 _y_3) (Math|Vector2D|BreakVector2D _holdingmouseposition))
  (bind _returnvalue (- _holdingmouseposition_2 _ontapmouseposition___2))
  (bind (_x_4 _y_4) (Math|Vector2D|BreakVector2D _returnvalue))
  (HUD|DrawRect "(R=0,G=0,B=0,A=1)" _x_2 _y_2 5.0 5.0)
  (HUD|DrawRect "(R=0,G=0,B=0,A=1)" _x_3 _y_3 5.0 5.0)
  (HUD|DrawRect "(R=0.224067,G=0.284232,B=0.896269,A=0.243000)" _x _y _x_4 _y_4))

(event EventOnInputTap
  (bind _returnvalue (Game|Player|GetOwningPlayerController))
  (bind (_locationx _locationy) (Game|Player|GetMousePosition _returnvalue))
  (for _array_element (Variables|Default|GetSelectedActors)
    (Class|SelectionInterface|OnSelectionLost(Message) _array_element))
  (Utilities|Array|Clear (Variables|Default|Getbuffer_selection))
  (Utilities|Array|Clear (Variables|Default|GetSelectedActors))
  (Utilities|Array|Clear (Variables|Default|GetFoundActors))
  (bind _output_get (Variables|Default|SetOnTapMousePosition%20	 (Math|Vector2D|MakeVector2D _locationx _locationy)))
  (Variables|Default|SetHoldingMousePosition _output_get)
  (Variables|Default|SetisDrawingSelection true))

(event EventOnInputHold
  (bind _returnvalue (Game|Player|GetOwningPlayerController))
  (bind (_locationx _locationy) (Game|Player|GetMousePosition _returnvalue))
  (Variables|Default|SetHoldingMousePosition (Math|Vector2D|MakeVector2D _locationx _locationy)))

(event EventOnInputHoldReleased
  (params (HoldTime :type Float%20%28single-precision%29))
  (Variables|Default|SetisDrawingSelection false)
  (bind _asrtsplayer_controller (Utilities|Casting|CastToRTSPlayerController (Game|Player|GetOwningPlayerController)))
  (Default|SetSelectedPawns _asrtsplayer_controller (Variables|Default|GetSelectedActors)))

(event EventDrawHUD
  (params (SizeX :type Integer) (SizeY :type Integer))
  (if (Variables|Default|GetisDrawingSelection)
    (Utilities|FlowControl|Sequence
      (:then_0
        (CallFunction|DrawMouseSelection))
      (:then_1
        (CallFunction|OnSelectionLost))
      (:then_2
        (bind _output_get (Variables|Default|Setbuffer_selection (Class|HUD|GetActorsinSelectionRectangle "/Script/Engine.Character" (Variables|Default|GetOnTapMousePosition%20	) (Variables|Default|GetHoldingMousePosition) false false)))
        (for _array_element _output_get
          (Utilities|Array|AddUnique (Variables|Default|GetFoundActors) _array_element)
          (for _array_element_2 (Variables|Default|GetFoundActors)
            (if (Utilities|DoesObjectImplementInterface _array_element_2 "/Game/blueprints/blueprints_for_RTS_camera/SelectionInterface.SelectionInterface_C")
              (Class|SelectionInterface|OnSelectionGained(Message) _array_element_2)
              (Utilities|Array|AddUnique (Variables|Default|GetSelectedActors) _array_element_2)))
          (for _array_element_3 (Variables|Default|GetSelectedActors)
            (Rendering|Debug|DrawDebugPoint (+ (Transformation|GetActorLocation _array_element_3) "0, 0,128.000000") 5e+01 "(R=1.000000,G=0.000000,B=0.024068,A=1.000000)" 0.0)))))))

(fn ConstructionScript)