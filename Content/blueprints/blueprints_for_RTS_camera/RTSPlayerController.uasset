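; RTS player controller that drives the camera pawn, unit selection and move orders, and creates the top bar and pause menu widgets.
; Tick runs a camera state machine for screen-edge scrolling and drag panning, which shifts the pawn by cursor ground-trace deltas.
; Select input sends tap, hold and release messages to the HUD.
; Short move clicks send selected pawns interface messages with two-column grid offsets around the traced cursor point, marked by debug spheres.
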(event Custom|UpdateSelection
  ;[1 1 1] сссс
  (if (Variables|Default|GetisHoldingInput)
    (Variables|Default|SetInputHoldingTime%20	 (+ (Variables|Default|GetInputHoldingTime%20	) (Variables|Default|GetDeltaTime)))
    (Class|InputInterface|OnInputHold(Message) (HUD|GetHUD))))

(event Custom|UpdateClickToMove
  ;[1 1 1] сссс
  (if (Variables|Default|GetWantToMove)
    (Variables|Default|SetMoveClickTime%20	 (+ (Variables|Default|GetMoveClickTime%20	) (Variables|Default|GetDeltaTime)))))

(event Custom|UpdateCamera
  (bind _returnvalue (Pawn|GetControlledPawn))
  ;[1 1 1] сссс
  (switch Utilities|FlowControl|Switch|SwitchonEInputType (Variables|Default|GetCurrentInputState)
    (:NewEnumerator0
      (bind _drag (CallFunction|IsScrolling :!label _label))
      (if (Utilities|Enum|NotEqual(Enum) _drag "NewEnumerator0")
        (bind _direction (CallFunction|GetScrollDirection))
        (Pawn|Input|AddMovementInput (Pawn|GetControlledPawn) _direction 1.0 false)
        (Variables|Default|SetCurrentInputState "NewEnumerator3")))
    (:NewEnumerator2
      (if (Variables|Default|GetisScrollingCamera%20	)
        (bind _delta (CallFunction|OnSwipeUpdate))
        (Transformation|SetActorLocation _returnvalue (+ _delta (Transformation|GetActorLocation _returnvalue)) false false)))
    (:NewEnumerator3
      (goto _label))))

(event EventTick
  (params (DeltaSeconds :type Float%20%28single-precision%29))
  ;[1 1 1] сссс
  (Variables|Default|SetDeltaTime DeltaSeconds)
  (CallFunction|UpdateCamera)
  (CallFunction|UpdateSelection)
  (CallFunction|UpdateClicktoMove))

(event EventBeginPlay
  ;[1 1 1] UI Ресурсов
  (bind _returnvalue (UserInterface|CreateWidget "/Game/UI/WP_UpBar.WP_UpBar_C"))
  (UserInterface|Viewport|AddtoViewport _returnvalue 0))

(event Input|ActionEvents|InputActionSelectInput
  (params (Key :type Key%20Structure :default "None"))
  ;[1 1 1] сссс
  (:Pressed
    (Class|InputInterface|OnInputTap(Message) (HUD|GetHUD))
    (Variables|Default|SetInputHoldingTime%20	 0.0)
    (Variables|Default|SetisHoldingInput true))
  (:Released
    (Class|InputInterface|OnInputHoldReleased(Message) (HUD|GetHUD) (Variables|Default|GetInputHoldingTime%20	))
    (Variables|Default|SetisHoldingInput false)))

(event Input|ActionEvents|InputActionPanCamera
  (params (Key :type Key%20Structure :default "None"))
  ;[1 1 1] сссс
  (:Pressed
    (CallFunction|OnSwipeStarted)
    (Variables|Default|SetCurrentInputState "NewEnumerator2")
    (Variables|Default|SetisScrollingCamera%20	 true))
  (:Released
    (CallFunction|OnSwipeEnded)
    (Variables|Default|SetCurrentInputState "NewEnumerator0")))

(event Input|ActionEvents|InputActionMovePawns
  (params (Key :type Key%20Structure :default "None"))
  ;[1 1 1] сссс
  (:Pressed
    (Variables|Default|SetMoveClickTime%20	 0.0)
    (Variables|Default|SetWantToMove true))
  (:Released
    (Variables|Default|SetWantToMove false)
    (if (< (Variables|Default|GetMoveClickTime%20	) 3.0)
      (for (_array_element _array_index) (Variables|Default|GetSelectedPawns)
        (bind _output_get (Variables|Default|SetMoveToLocation%20	 (+ (Math|Vector|MakeVector (* (/ _array_index 2) 1.5e+02) (* (Math|Integer|%(Integer) _array_index 2) 1.5e+02) 0.0) (.Location (Collision|BreakHitResult (.HitResult (Game|Player|GetHitResultUnderCursorbyChannel "TraceTypeQuery3" true)))))))
        (Class|IMovement|MovetoMouseLoc(Message) _array_element _output_get)
        (Rendering|Debug|DrawDebugSphere _output_get 25.0 30 "(R=1.000000,G=0.819536,B=0.137427,A=1.000000)" 5.0)))))

(event Input|KeyboardEvents|P
  (params (Key :type Key%20Structure :default "None"))
  ;[1 1 1] Для меню паузы
  (:Pressed
    (bind _returnvalue (UserInterface|CreateWidget "/Game/UI/PauseMenu.PauseMenu_C"))
    (UserInterface|Viewport|AddtoViewport _returnvalue 0)))

(fn ConstructionScript)

(fn OnSwipeStarted
  (Variables|Default|SetStartSwipeCoords%20	 (.Location (Collision|BreakHitResult (.HitResult (Game|Player|GetHitResultUnderCursorbyChannel "TraceTypeQuery3" true))))))

(fn OnSwipeEnded
  (Variables|Default|SetEndSwipeCoords%20	 (.Location (Collision|BreakHitResult (.HitResult (Game|Player|GetHitResultUnderCursorbyChannel "TraceTypeQuery3" true)))))
  (Variables|Default|SetStartSwipeCoords%20	 "0, 0, 0"))

(fn OnSwipeUpdate
  (LocalVariables|SetLocalNewSwipeCoords (.Location (Collision|BreakHitResult (.HitResult (Game|Player|GetHitResultUnderCursorbyChannel "TraceTypeQuery3" true)))))
  (bind _output_get (LocalVariables|SetLocalDelta (Math|Vector|MakeVector (.X (Math|Vector|BreakVector (- (Variables|Default|GetStartSwipeCoords%20	) (LocalVariables|GetLocalNewSwipeCoords)))) (.Y (Math|Vector|BreakVector (- (Variables|Default|GetStartSwipeCoords%20	) (LocalVariables|GetLocalNewSwipeCoords)))) 0.0)))
  (return _output_get))

(fn IsScrolling
  (bind (_locationx _locationy) (Game|Player|GetMousePosition))
  (bind _returnvalue (Viewport|GetViewportSize))
  (bind (_locationx_2 _locationy_2) (Game|Player|GetMousePosition))
  (bind _returnvalue_2 (Viewport|GetViewportSize))
  (bind (_locationx_3 _locationy_3) (Game|Player|GetMousePosition))
  (bind (_x _y) (Math|Vector2D|BreakVector2D _returnvalue_2))
  (bind (_x_2 _y_2) (Math|Vector2D|BreakVector2D _returnvalue))
  (bind _returnvalue_3 (* _x_2 0.1))
  (bind _returnvalue_4 (* _y_2 0.1))
  (bind _returnvalue_5 (< _locationy_3 _returnvalue_4))
  (bind _returnvalue_6 (< _locationx_3 _returnvalue_3))
  (Utilities|FlowControl|Sequence
    (:then_0
      (if _returnvalue_6
        (LocalVariables|SetLocal%20Drag "NewEnumerator2")))
    (:then_1
      (if (and (not _returnvalue_6) (> _locationx_2 (* _x 0.9)))
        (LocalVariables|SetLocal%20Drag "NewEnumerator1")))
    (:then_2
      (if _returnvalue_5
        (LocalVariables|SetLocal%20Drag "NewEnumerator3")))
    (:then_3
      (if (and (not _returnvalue_5) (> _locationy_2 (* _y 0.9)))
        (LocalVariables|SetLocal%20Drag "NewEnumerator4")))
    (:then_4
      (if (and (== _locationx 0.0) (== _locationy 0.0))
        (LocalVariables|SetLocal%20Drag "NewEnumerator0")))
    (:then_5
      (return (LocalVariables|GetLocal%20Drag)))))

(fn SetSelectedPawns
  (params (SelectedPawns :type Array%20of%20Actor%20Object%20References))
  (Variables|Default|SetSelectedPawns SelectedPawns))

(fn GetScrollDirection
  (bind (_locationx _locationy) (Game|Player|GetMousePosition))
  (bind _returnvalue (Viewport|GetViewportSize))
  (bind _returnvalue_2 (Math|Vector2D|MakeVector2D _locationx _locationy))
  (bind _returnvalue_3 (/ _returnvalue 2.0))
  (bind _returnvalue_4 (- _returnvalue_2 _returnvalue_3))
  (bind _returnvalue_5 (Math|Conversions|ToVector(Vector2D) _returnvalue_4))
  (bind _returnvalue_6 (* _returnvalue_5 -1.0))
  (bind _returnvalue_7 (Math|Vector|ClampVectorSize _returnvalue_6 0.2 1.0))
  (bind (_x _y) (Math|Vector|BreakVector _returnvalue_7))
  (return (Math|Vector|MakeVector (* _y -1.0) _x 0.0)))